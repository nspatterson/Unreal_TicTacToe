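; BP_Tile is a tile actor that shows whether the local player or someone else has claimed it.
; A RepNotify on ClaimedBy compares the stored name with the name from player controller 0's PlayerState.
; It sets the Cube's material to P0Mat on a match and P1Mat otherwise, so the color is relative to each viewer.
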(event EventOnRepClaimedby
  (bind _name (CallFunction|GetPlayerName))
  (if (== _name (Variables|Default|GetClaimedBy))
    (CallFunction|SetMaterial (Variables|Default|GetP0_Mat))
    (else
      (CallFunction|SetMaterial (Variables|Default|GetP1_Mat)))))

(event EventTick
  (params (DeltaSeconds :type Float%20%28single-precision%29)))

(fn ConstructionScript)

(fn GetPlayerName
  (return (PlayerState|GetPlayerName (Variables|/Script/Engine.Controller|GetPlayerState (Game|GetPlayerController 0)))))

(fn SetMaterial
  (params (Material :type Material%20Object%20Reference))
  (Rendering|Material|SetMaterial (Variables|Default|GetCube) 0 Material))