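; BP_Tile2 is a claimable tile whose cube changes color to show which player claimed it.
; The replicated ClaimedBy name's OnRep compares it with the local player's name to pick the P0 or P1 color.
; It writes that color and the current game time to material parameters ClaimColor and StartTime, likely for a timed shader transition.
; A SetMaterial helper swaps the cube's material, and the P1 branch prints a leftover debug string.
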(event EventOnRepClaimedby
  (bind _name (CallFunction|GetPlayerName))
  (if (== _name (Variables|Default|GetClaimedBy))
    (Rendering|Material|SetScalarParameterValueonMaterials (Variables|Default|GetCube) "StartTime" (Utilities|Time|GetGameTimeinSeconds))
    (Rendering|Material|SetVectorParameterValueonMaterials (Variables|Default|GetCube) "ClaimColor" (Variables|Default|GetP0_Color_Vector))
    (else
      (Rendering|Material|SetScalarParameterValueonMaterials (Variables|Default|GetCube) "StartTime" (Utilities|Time|GetGameTimeinSeconds))
      (Rendering|Material|SetVectorParameterValueonMaterials (Variables|Default|GetCube) "ClaimColor" (Variables|Default|GetP1_Color_Vector))
      (Development|PrintString "cum"))))

(fn ConstructionScript)

(fn GetPlayerName
  (return (PlayerState|GetPlayerName (Variables|/Script/Engine.Controller|GetPlayerState (Game|GetPlayerController 0)))))

(fn SetMaterial
  (params (Material :type Material%20Object%20Reference))
  (Rendering|Material|SetMaterial (Variables|Default|GetCube) 0 Material))