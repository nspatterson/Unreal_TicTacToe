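; BP_Tile4 is a claimable board tile that shows an X or O decal, as in tic-tac-toe.
; When the replicated ClaimedBy value changes, it compares it with the first player controller's player name, choosing X for a match and O otherwise.
; The chosen decal gets a dynamic material stamped with the current game time as StartTime.
; Older cube color-tinting logic remains disconnected, and a helper swaps the cube's material.
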(event EventOnRepClaimedby
  (bind _name (CallFunction|GetPlayerName))
  (if (== _name (Variables|Default|GetClaimedBy))
    (bind _returnvalue (Rendering|Material|CreateDynamicMaterialInstance (Variables|Default|GetDecal_X) :!class /Script/Engine.DecalComponent))
    (Rendering|Material|SetScalarParameterValue _returnvalue "StartTime" (Utilities|Time|GetGameTimeinSeconds) :!class /Script/Engine.MaterialInstanceDynamic)
    (else
      (bind _returnvalue_2 (Rendering|Material|CreateDynamicMaterialInstance (Variables|Default|GetDecal_O) :!class /Script/Engine.DecalComponent))
      (Rendering|Material|SetScalarParameterValue _returnvalue_2 "StartTime" (Utilities|Time|GetGameTimeinSeconds) :!class /Script/Engine.MaterialInstanceDynamic))))

(fn ConstructionScript)

(fn GetPlayerName
  (return (PlayerState|GetPlayerName (Variables|/Script/Engine.Controller|GetPlayerState (Game|GetPlayerController 0)))))

(fn SetMaterial
  (params (Material :type Material%20Object%20Reference))
  (Rendering|Material|SetMaterial (Variables|Default|GetCube) 0 Material))